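; Base first-person weapon actor, attached to BP_FirstPersonCharacter, handling single or automatic fire, reloading and an ammo widget.
; Each shot plays paired arm and gun animations, spends ammo, shakes the camera and drives timeline-based recoil.
; Hitscan traces from the camera, aims the muzzle flash at that point and picks impact effects from component tags, without applying damage.
; Reload animations differ for empty and partial magazines; Equip passes the ADS offset to the player.
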(event `self.ReceiveBeginPlay`
  (bind _asbp_first_person_character (cast `/Game/FirstPerson/Blueprints/BP_FirstPersonCharacter` (`self.GetParentActor`)))
  (set `self.PlayerRef` _asbp_first_person_character)
  (set `self.CurrentAmmo` (`self.MagSize`))
  (`self.UpdateAmmoDisplay`))

(event `Stow`)

(event `Fire`
  (switch `/Game/Weapons/E_FireMode` (`self.FireMode`)
    (:`NewEnumerator0`
      (`self.StartFire`)
      (`self.StopFire`))
    (:`NewEnumerator1`
      (if (`/Game/FirstPerson/Blueprints/BP_FirstPersonCharacter.IsShooting` (`self.PlayerRef`)) :!label _label
        (`self.StartFire`)
        (`KismetSystemLibrary.Delay` (`self.FireDelay`))
        (goto _label)))))

(event `Reload`
  (bind (_playeranimmontages_firemontage _playeranimmontages_firelastmontage _playeranimmontages_reloadmontage _playeranimmontages_reloadnotfullmontage) (break `/Game/FirstPerson/Structs/S_WeaponMontages` (`self.PlayerAnimMontages`)))
  (bind (_playeranimmontages_firemontage_2 _playeranimmontages_firelastmontage_2 _playeranimmontages_reloadmontage_2) (break `/Game/FirstPerson/Structs/S_WeaponMontages` (`self.PlayerAnimMontages`)))
  (bind (_gunanimmontages_firemontage _gunanimmontages_firelastmontage _gunanimmontages_reloadmontage _gunanimmontages_reloadnotfullmontage) (break `/Game/FirstPerson/Structs/S_WeaponMontages` (`self.GunAnimMontages`)))
  (bind (_gunanimmontages_firemontage_2 _gunanimmontages_firelastmontage_2 _gunanimmontages_reloadmontage_2) (break `/Game/FirstPerson/Structs/S_WeaponMontages` (`self.GunAnimMontages`)))
  (if (not (`self.IsReloading`))
    (set `self.IsReloading` true)
    (if (== (`self.CurrentAmmo`) 0)
      (`|PlayMontage` (`/Game/FirstPerson/Blueprints/BP_FirstPersonCharacter.FirstPersonMesh` (`self.PlayerRef`)) _playeranimmontages_reloadmontage_2
        (:`then`
          (`SkeletalMeshComponent.PlayAnimation` (`self.WeaponMesh`) _gunanimmontages_reloadmontage_2 false))
        (:`OnBlendOut`
          (set `self.CurrentAmmo` (`self.MagSize`) :!label _label_2)
          (`self.UpdateAmmoDisplay`)
          (set `self.IsReloading` false))
        (:`OnInterrupted`
          (`KismetSystemLibrary.RetriggerableDelay` 3.75)
          (set `self.IsReloading` false)))
      (else
        (`|PlayMontage` (`/Game/FirstPerson/Blueprints/BP_FirstPersonCharacter.FirstPersonMesh` (`self.PlayerRef`)) _playeranimmontages_reloadnotfullmontage
          (:`then`
            (`SkeletalMeshComponent.PlayAnimation` (`self.WeaponMesh`) _gunanimmontages_reloadnotfullmontage false))
          (:`OnBlendOut`
            (goto _label_2))
          (:`OnInterrupted`
            (`KismetSystemLibrary.RetriggerableDelay` 3.0)
            (set `self.IsReloading` false)))))))

(event `StartFire`
  (bind _returnvalue (`GameplayStatics.GetPlayerController` 0))
  (bind _playeranimmontages_firemontage (break `/Game/FirstPerson/Structs/S_WeaponMontages` (`self.PlayerAnimMontages`)))
  (bind (_gunanimmontages_firemontage _gunanimmontages_firelastmontage) (break `/Game/FirstPerson/Structs/S_WeaponMontages` (`self.GunAnimMontages`)))
  (bind _gunanimmontages_firemontage_2 (break `/Game/FirstPerson/Structs/S_WeaponMontages` (`self.GunAnimMontages`)))
  (bind (_playeranimmontages_firemontage_2 _playeranimmontages_firelastmontage) (break `/Game/FirstPerson/Structs/S_WeaponMontages` (`self.PlayerAnimMontages`)))
  (bind _returnvalue_2 (- (`self.CurrentAmmo`) 1))
  (if (> _returnvalue_2 0)
    (`GameplayStatics.PlaySoundAtLocation` (`self.FireSound`) (`self.K2_GetActorLocation`) (struct) 1.0 1.0 0.0 null null null null)
    (`|PlayMontage` (`/Game/FirstPerson/Blueprints/BP_FirstPersonCharacter.FirstPersonMesh` (`self.PlayerRef`)) _playeranimmontages_firemontage
      (:`then`
        (`SkeletalMeshComponent.PlayAnimation` (`self.WeaponMesh`) _gunanimmontages_firemontage_2 false)
        (`/Engine/EditorBlueprintResources/StandardMacros.DecrementInt` (`self.CurrentAmmo`) :!label _label_3
          (:`  `
            (`self.FireHitScan` false)
            (`self.UpdateAmmoDisplay`)
            (`GameplayStatics.PlayWorldCameraShake` "/Game/FirstPerson/CameraShake/CS_Fire.CS_Fire_C" (`self.K2_GetActorLocation` (`self.PlayerRef`)) 0.0 100.0)
            (bind (_direction _pitchrecoil _yawrecoil) (`Timeline|TL_Recoil` :!label _label_4)
              (:`Update`
                (switch `ETimelineDirection` _direction
                  (:`Forward`
                    (`PlayerController.AddPitchInput` _returnvalue _pitchrecoil)
                    (`PlayerController.AddYawInput` _returnvalue _yawrecoil)))))))))
    (elif (== _returnvalue_2 0)
      (`GameplayStatics.PlaySoundAtLocation` (`self.FireSound`) (`self.K2_GetActorLocation`) (struct) 1.0 1.0 0.0 null null null null)
      (`|PlayMontage` (`/Game/FirstPerson/Blueprints/BP_FirstPersonCharacter.FirstPersonMesh` (`self.PlayerRef`)) _playeranimmontages_firelastmontage
        (:`then`
          (`SkeletalMeshComponent.PlayAnimation` (`self.WeaponMesh`) _gunanimmontages_firelastmontage false)
          (goto _label_3)))
      (else
        (`GameplayStatics.PlaySoundAtLocation` (`self.EmptySound`) (`self.K2_GetActorLocation`) (struct) 1.0 1.0 0.0 null null null null)
        (bind _aswbp_ammo_display (cast `/Game/Weapons/Widgets/WBP_AmmoDisplay` (`WidgetComponent.GetWidget` (`self.AmmoDisplay`))))
        (`/Game/Weapons/Widgets/WBP_AmmoDisplay.AmmoError` _aswbp_ammo_display)
        (`self.StopFire`)))))

(event `StopFire`
  (if (`|EnumEquality` (`self.FireMode`) "NewEnumerator0")
    (`KismetSystemLibrary.Delay` 0.2)
    (goto _label_4 :!via `Reverse`)
    (else
      (goto _label_4 :!via `Reverse`))))

(event `Equip`
  (set `/Game/FirstPerson/Blueprints/BP_FirstPersonCharacter.ADSOffset` (`self.ADSOffset`) (`self.PlayerRef`)))

(fn `FireHitScan`
  (params (DrawDebug :type Boolean))
  (locals (HitInfo :type "HitResult Structure"))
  (bind (_hitinfo_bblockinghit _hitinfo_binitialoverlap _hitinfo_time _hitinfo_distance _hitinfo_location _hitinfo_impactpoint _hitinfo_normal _hitinfo_impactnormal _hitinfo_physmat _hitinfo_hitactor _hitinfo_hitcomponent) (`GameplayStatics.BreakHitResult` (`local.HitInfo`)))
  (bind _returnvalue (`SceneComponent.GetSocketLocation` (`self.WeaponMesh`) "Muzzle"))
  (bind _firstpersoncamera (`/Game/FirstPerson/Blueprints/BP_FirstPersonCharacter.FirstPersonCamera` (`self.PlayerRef`)))
  (bind _returnvalue_2 (`SceneComponent.K2_GetComponentLocation` _firstpersoncamera))
  (bind _outhit (`KismetSystemLibrary.LineTraceSingle` _returnvalue_2 (+ _returnvalue_2 (* (`SceneComponent.GetForwardVector` _firstpersoncamera) (`self.Range`))) "TraceTypeQuery1" false (`|MakeArray` self (`self.PlayerRef`) :!type "Actor Object Reference")))
  (set `local.HitInfo` _outhit)
  (bind (_bblockinghit _binitialoverlap _time _distance _location _impactpoint _normal _impactnormal _physmat _hitactor _hitcomponent _hitbonename _bonename _hititem _elementindex _faceindex _tracestart _traceend) (`GameplayStatics.BreakHitResult` _outhit))
  (bind _returnvalue_3 (`KismetMathLibrary.SelectVector` _location _traceend _bblockinghit))
  (`KismetSystemLibrary.LineTraceSingle` :`Start` (`SceneComponent.GetSocketLocation` (`self.WeaponMesh`) "Muzzle") :`End` _returnvalue_3 :`TraceChannel` "TraceTypeQuery1" :`DrawDebugType` (select `bool` (`local.DrawDebug`) :`true` "ForDuration" :!type "EDrawDebugTrace Enum"))
  (`NiagaraFunctionLibrary.SpawnSystemAttached` "/Game/Weapons/MuzzleFlash/NS_MuzzleFlash.NS_MuzzleFlash" (`self.WeaponMesh`) "Muzzle" _returnvalue (`KismetMathLibrary.FindLookAtRotation` _returnvalue _returnvalue_3) "KeepWorldPosition" true)
  (if _hitinfo_bblockinghit
    (`self.HitEffect` _hitinfo_hitcomponent _hitinfo_location _hitinfo_normal))
  (return))

(fn `HitEffect`
  (params (HitComponent :type "ActorComponent Object Reference") (HitLocation :type "Vector Structure") (HitNormal :type "Vector Structure"))
  (locals (Tag :type Name))
  (bind _hitlocation (`local.HitLocation`))
  (bind _hitnormal (`local.HitNormal`))
  (for _array_element (`ActorComponent.ComponentTags` HitComponent)
    (set `local.Tag` _array_element))
  (switch `name` (`local.Tag`)
    (:`Default`
      (`self.SpawnHitEffect` "/Game/Weapons/HitEffects/Niagara/NS_Hit_Concrete.NS_Hit_Concrete" "/Game/Weapons/HitEffects/Audio/SC_Hit_Concrete.SC_Hit_Concrete" _hitlocation _hitnormal :!label _label))
    (:`Flesh`
      (`self.SpawnHitEffect` "/Game/Weapons/HitEffects/Niagara/NS_Hit_Blood.NS_Hit_Blood" "/Game/Weapons/HitEffects/Audio/SC_Hit_Blood.SC_Hit_Blood" _hitlocation _hitnormal))
    (:`Metal`
      (`self.SpawnHitEffect` "/Game/Weapons/HitEffects/Niagara/NS_Hit_Metal.NS_Hit_Metal" "/Game/Weapons/HitEffects/Audio/SC_Hit_Metal.SC_Hit_Metal" _hitlocation _hitnormal))
    (:`Concrete`
      (goto _label)))
  (return))

(fn `SpawnHitEffect`
  (params (HitEffect :type "NiagaraSystem Object Reference") (HitSound :type "SoundCue Object Reference") (HitLocation :type "Vector Structure") (HitNormal :type "Vector Structure"))
  (`NiagaraFunctionLibrary.SpawnSystemAtLocation` HitEffect HitLocation (`KismetMathLibrary.Conv_VectorToRotator` HitNormal))
  (`GameplayStatics.PlaySoundAtLocation` HitSound HitLocation (struct) 1.0 1.0 0.0 null null null null))

(fn `UpdateAmmoDisplay`
  (bind _aswbp_ammo_display (cast `/Game/Weapons/Widgets/WBP_AmmoDisplay` (`WidgetComponent.GetWidget` (`self.AmmoDisplay`))))
  (set `/Game/Weapons/Widgets/WBP_AmmoDisplay.CurrentAmmo` (`self.CurrentAmmo`) _aswbp_ammo_display)
  (set `/Game/Weapons/Widgets/WBP_AmmoDisplay.MagSize` (`self.MagSize`) _aswbp_ammo_display))

(fn `UserConstructionScript`
  (`SkeletalMeshComponent.SetSkeletalMeshAsset` (`self.WeaponMesh`) (`self.Mesh`)))