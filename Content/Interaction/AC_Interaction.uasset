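; Actor component that lets its owner detect and use interactable actors the player camera looks at.
; Every tick it runs a short Visibility line trace from the camera and stores any hit actor implementing BI_Interaction.
; It shows that actor's interaction text in WBP_Interaction, clearing both when the target is lost.
; The IA_Interact input sends InteractMessage to the stored actor, passing the component's owner.
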(event `self.ReceiveBeginPlay`
  (bind _widgetref (`/Game/Interaction/BML_AC_Interaction.GetWidgetRef` "/Game/Interaction/WBP_Interaction.WBP_Interaction_C")
    (:`True`
      (bind _aswbp_interaction (cast `/Game/Interaction/WBP_Interaction` _widgetref))
      (set `self.WBPRef` _aswbp_interaction))))

(event `self.ReceiveTick`
  (params (DeltaSeconds :type "Float (single-precision)"))
  (`self.InteractionTrace`))

(event `EnhancedInput|/Game/FirstPerson/Input/Actions/IA_Interact`
  (params (ActionValue :type Boolean) (ElapsedSeconds :type "Float (double-precision)") (TriggeredSeconds :type "Float (double-precision)") (InputAction :type "InputAction Object Reference" :default "/Game/FirstPerson/Input/Actions/IA_Interact.IA_Interact"))
  (:`Triggered`
    (bind _interactableactor (`self.InteractableActor`)
      (:`then`
        (message `/Game/Interaction/BI_Interaction.Interact` _interactableactor (`self.GetOwner`)))
      (:`else`))))

(fn `InteractionTrace`
  (bind _returnvalue (`GameplayStatics.GetPlayerCameraManager` 0))
  (bind _returnvalue_2 (`Actor.K2_GetActorLocation` _returnvalue))
  (bind (_outhit _returnvalue_3) (`KismetSystemLibrary.LineTraceSingle` _returnvalue_2 (+ _returnvalue_2 (* (`Actor.GetActorForwardVector` _returnvalue) 250.0)) "TraceTypeQuery1"))
  (if _returnvalue_3
    (bind (_bblockinghit _binitialoverlap _time _distance _location _impactpoint _normal _impactnormal _physmat _hitactor) (`GameplayStatics.BreakHitResult` _outhit))
    (if (`KismetSystemLibrary.DoesImplementInterface` _hitactor "/Game/Interaction/BI_Interaction.BI_Interaction_C")
      (bind _output_get (set `self.InteractableActor` _hitactor))
      (bind _interactiontext (message `/Game/Interaction/BI_Interaction.GetInteractData` _output_get))
      (`/Game/Interaction/WBP_Interaction.UpdateInteraction` (`self.WBPRef`) true _interactiontext)
      (else
        (`self.InteractableActor` :!label _label
          (:`then`
            (set `self.InteractableActor` null)
            (`/Game/Interaction/WBP_Interaction.UpdateInteraction` (`self.WBPRef`) false ""))
          (:`else`))))
    (else
      (goto _label))))